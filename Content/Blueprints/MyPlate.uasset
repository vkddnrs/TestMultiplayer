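; A plate actor that moves vertically when stepped on and shows a message widget naming the character on it.
; Each begin overlap restarts the Plate_move timeline, which offsets Z from the current location.
; An IsEnd flag gates widget creation, which runs only with authority after a busy-wait loop on an externally supplied PlayerName.
; End overlap removes the widget, and PullMessage removes or recreates it according to IsEnd.
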(event Collision|EventActorBeginOverlap
  (params (OtherActor :type Actor%20Object%20Reference))
  (Utilities|FlowControl|Sequence
    (:then_0
      ;[1 1 1] Поднимаем - опускаем плиту
      (Variables|Default|SetBeginPos (Transformation|GetActorLocation))
      (if true
        (bind _newtrack_2 (Timeline|Plate_move PlayFromStart)
          (:Update
            (Transformation|SetActorLocation (Math|Vector|MakeVector (.x (Variables|Default|GetBeginPos)) (.y (Variables|Default|GetBeginPos)) (+ (.z (Variables|Default|GetBeginPos)) (* _newtrack_2 1e+01))) false false)))))
    (:then_1
      ;[1 1 1] Добавляем и удаляем виджеты с именем Персонажа, взобравшегося на плиту последним. Конечно, это не самое лучшее решение, но пока то, что могу сделать.
      (if (Variables|Default|Getis_end)
        (Variables|Default|Setis_end false)
        (Networking|SwitchHasAuthority
          (:Authority
            (while (Utilities|Enum|Equal(Enum) (Variables|Default|GetPlayerName) "")
              _)
            (bind _returnvalue (UserInterface|CreateWidget "/Game/GUI/Message.Message_C" 0 (Variables|Default|GetPlayerName)))
            (bind _output_get (Variables|Default|SetMessage _returnvalue))
            (UserInterface|Viewport|AddtoViewport _output_get 0)))))))

(event EventEndOverlap
  (bind _message (Variables|Default|GetMessage))
  ;[1 1 1] Добавляем и удаляем виджеты с именем Персонажа, взобравшегося на плиту последним. Конечно, это не самое лучшее решение, но пока то, что могу сделать.
  (if (not (Variables|Default|Getis_end))
    (Variables|Default|Setis_end true)
    (Utilities|IsValid _message
      (:Is%20Valid
        (Widget|RemovefromParent _message)))))

(event EventPullMessage
  ;[1 1 1] Добавляем и удаляем виджеты с именем Персонажа, взобравшегося на плиту последним. Конечно, это не самое лучшее решение, но пока то, что могу сделать.
  (if (Variables|Default|Getis_end)
    (Widget|RemovefromParent (Variables|Default|GetMessage))
    (else
      (bind _returnvalue (UserInterface|CreateWidget "/Game/GUI/Message.Message_C" 0 (Variables|Default|GetPlayerName)))
      (bind _output_get (Variables|Default|SetMessage _returnvalue))
      (UserInterface|Viewport|AddtoViewport _output_get 0))))

(fn ConstructionScript)