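; Light bulb actor that lights up and goes dark through the EmissiveColor parameter of a dynamic material created on its sphere at construction.
; OnRepColor applies ColorEmissive to the material, as does Tick every frame while IsLighting is true.
; When unlit, Tick uses a DoOnce to set the color to black on the authority only.
; OnLightEvent resets that DoOnce so the bulb can be switched off again.
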(event EventBeginPlay)

(event Collision|EventActorBeginOverlap
  (params (OtherActor :type Actor%20Object%20Reference)))

(event EventTick
  (params (DeltaSeconds :type Float%20%28single-precision%29))
  ;[1 1 1] Зажигаем / гасим лампочку
  (if (Variables|Default|GetIsLighting)
    (Rendering|Material|SetVectorParameterValue (Variables|Default|GetDynamicMaterial) "EmissiveColor" (Variables|Default|GetColorEmissive) :!class /Script/Engine.MaterialInstanceDynamic)
    (else
      (Utilities|FlowControl|DoOnce false
        (:Completed
          (Networking|SwitchHasAuthority
            (:Authority
              (bind _output_get (Variables|Default|SetColorEmissive ""))
              (Rendering|Material|SetVectorParameterValue (Variables|Default|GetDynamicMaterial) "EmissiveColor" _output_get :!class /Script/Engine.MaterialInstanceDynamic))))))))

(event EventOnRepColor
  ;[1 1 1] Зажигаем / гасим лампочку
  (Rendering|Material|SetVectorParameterValue (Variables|Default|GetDynamicMaterial) "EmissiveColor" (Variables|Default|GetColorEmissive) :!class /Script/Engine.MaterialInstanceDynamic))

(event EventOnLightEvent
  ;[1 1 1] Зажигаем / гасим лампочку
  (Utilities|FlowControl|DoOnce false) ; enters at Reset
)

(fn ConstructionScript
  (bind _returnvalue (Rendering|Material|CreateDynamicMaterialInstance (Variables|Default|GetSphere) 0 0 "None" :!class /Script/Engine.PrimitiveComponent))
  (Variables|Default|SetDynamicMaterial _returnvalue))